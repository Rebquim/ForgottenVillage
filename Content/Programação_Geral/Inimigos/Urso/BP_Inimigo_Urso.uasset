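; Bear enemy Blueprint that roams the map, chases pawns it sees and damages the player.
; It loops AIMoveTo to random reachable points around itself.
; On PawnSensing sight it moves to the seen pawn, applies damage to player 0 on arrival, and resumes wandering via a retriggerable delay.
; Tick shows a widget health bar when the player is near, rotating it toward them and updating its fill from current health.
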(event `Andar Pelo Mapa`
  ;[1 1 1] Andar pelo mapa de modo aleatorio
  (`|AIMoveTo` self (`NavigationSystemV1.K2_GetRandomReachablePointInRadius` (`self.K2_GetActorLocation`) 3000.0 null null) null
    (:`OnSuccess`
      (`KismetSystemLibrary.Delay` 0.2)
      (`self.Andar Pelo Mapa`))))

(event `self.ReceiveBeginPlay`
  ;[1 1 1] Andar pelo mapa de modo aleatorio
  (`self.Andar Pelo Mapa`))

(event `self.PawnSensing.OnSeePawn`
  (params (Pawn :type "Pawn Object Reference"))
  ;[1 1 1] Seguir o Player que ver
  (`|ExecutionSequence`
    (:`then_0`
      (`|AIMoveTo` self (0.0 0.0 0.0) Pawn 10.0
        (:`OnSuccess`
          (`GameplayStatics.ApplyDamage` (`GameplayStatics.GetPlayerCharacter` 0) 50.0))))
    (:`then_1`
      (`KismetSystemLibrary.RetriggerableDelay` 1.0)
      (`self.Andar Pelo Mapa`))))

(event `self.ReceiveTick`
  (params (DeltaSeconds :type "Float (single-precision)"))
  (bind _barra_de_vida (`self.Barra de vida`))
  (bind _barra_de_vida_2 (`self.Barra de vida`))
  ;[1 1 1] Barra de vida do inimigo
  (if (< (`KismetMathLibrary.VSize` (- (`self.K2_GetActorLocation` (`GameplayStatics.GetPlayerCharacter` 0)) (`self.K2_GetActorLocation`))) 2000.0)
    (`SceneComponent.SetVisibility` _barra_de_vida true false)
    (`SceneComponent.K2_SetWorldRotation` _barra_de_vida_2 (`KismetMathLibrary.FindLookAtRotation` (`self.K2_GetActorLocation`) (`self.K2_GetActorLocation` (`GameplayStatics.GetPlayerCharacter` 0))) false false)
    (bind _aswb_barra_de_vida_inimigo_urso (cast `/Game/Programação_Geral/Inimigos/Urso/WB_Barra_de_Vida_Inimigo_Urso` (`WidgetComponent.GetWidget` _barra_de_vida_2)))
    (`ProgressBar.SetPercent` (`/Game/Programação_Geral/Inimigos/Urso/WB_Barra_de_Vida_Inimigo_Urso.Barradevidadoinimigourso` _aswb_barra_de_vida_inimigo_urso) (/ (`self.Vida Atual`) 100.0))
    (else
      (`SceneComponent.SetVisibility` _barra_de_vida false false))))

(fn `UserConstructionScript`)